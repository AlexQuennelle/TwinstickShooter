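; BP_EnemySpawner is a spawner actor that adds BP_EnemyCharacter enemies to the level, up to a population cap.
; Its SpawnEnemy event counts every enemy of that class in the level and, while below MaxEnemies, spawns one AI pawn at a random point inside the SpawnVolume box.
; Nothing in this graph calls the event, and the construction script is empty.
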(event `SpawnEnemy`
  (bind _outactors (`GameplayStatics.GetAllActorsOfClass` "/Game/Blueprints/BP_EnemyCharacter.BP_EnemyCharacter_C"))
  (if (< (`KismetArrayLibrary.Array_Length` _outactors) (`self.MaxEnemies`))
    (`AIBlueprintHelperLibrary.SpawnAIFromClass` "/Game/Blueprints/BP_EnemyCharacter.BP_EnemyCharacter_C" null (`KismetMathLibrary.RandomPointInBoundingBox` (`SceneComponent.K2_GetComponentLocation` (`self.SpawnVolume`)) (`BoxComponent.GetScaledBoxExtent` (`self.SpawnVolume`))) (struct) false null)))

(fn `UserConstructionScript`)