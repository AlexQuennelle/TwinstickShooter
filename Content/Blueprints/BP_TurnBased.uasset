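; Turn manager Blueprint that runs initiative-ordered combat between player and enemy characters.
; On BeginPlay it enables the cursor, gathers all BP_Basecharacter actors, rolls random initiatives, sorts them ascending with recursive Quicksort and starts the first turn.
; AdvanceTurn cycles through combatants, skipping the dead.
; CombattantDied prints the winner if survivors share one class, otherwise regathers, rerolling initiative, and advances from the current combatant.
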(event Custom|Advance%20Turn
  ;[0.15 0.15 0.15 0.5] Increment and start the next turn
  (bind _output_get (Variables|Default|SetTurnIndex (|(({0B681E5D-42CB-167A-2EFB-DF8904E41FED}+1)%count) (Utilities|Array|Length (Variables|Default|GetCombatants)))))
  (if (Default|IsDead (Utilities|Array|Get(acopy) (Variables|Default|GetCombatants) _output_get))
    (CallFunction|AdvanceTurn)
    (else
      (Default|StartTurn (Utilities|Array|Get(acopy) (Variables|Default|GetCombatants) _output_get)))))

(event EventBeginPlay
  (Utilities|FlowControl|Sequence
    (:then_0
      ;[0.15 0.15 0.15 0.5] Setup
      (Variables|/Script/Engine.PlayerController|SetbShowMouseCursor (Game|GetPlayerController 0) true)
      (Variables|/Script/Engine.PlayerController|SetbEnableTouchOverEvents (Game|GetPlayerController 0) true))
    (:then_1
      ;[0.15 0.15 0.15 0.5] Kickstart turn system
      (bind _output_get (CallFunction|GatherCombattants))
      (Default|StartTurn (Utilities|Array|Get(acopy) _output_get)))))

(fn ConstructionScript)

(fn Quicksort
  (params (Input%20list :type Array%20of%20BP%20Basecharacter%20Object%20References))
  (bind _output_get (LocalVariables|SetArray Input%20list))
  ;[0.15 0.15 0.15 0.5] Abort if input array has 2 or fewer elements
  (if (>= (Utilities|Array|Length _output_get) 2)
    ;[0.15 0.15 0.15 0.5] Isolate the 'pivot' element to serve as a reference point
    (LocalVariables|SetPivotInitiative (Variables|/Game/Blueprints/BP_Basecharacter.BP_Basecharacter_C|GetInitiative (Utilities|Array|Get(acopy) (LocalVariables|GetArray) (Utilities|Array|LastIndex (LocalVariables|GetArray)))))
    (LocalVariables|SetPivot (Utilities|Array|Get(acopy) (LocalVariables|GetArray) (Utilities|Array|LastIndex (LocalVariables|GetArray))))
    (Utilities|Array|RemoveIndex (LocalVariables|GetArray) (Utilities|Array|LastIndex (LocalVariables|GetArray)))
    ;[0.15 0.15 0.15 0.5] Loop through remaining array
    (for _array_element (LocalVariables|GetArray)
      ;;[0.15 0.15 0.15 0.5] Compare each element to the 'pivot'
      (if (>= (Variables|/Game/Blueprints/BP_Basecharacter.BP_Basecharacter_C|GetInitiative _array_element) (LocalVariables|GetPivotInitiative))
        ;;[0.15 0.15 0.15 0.5] Add elements to separate lists based on that comparison
        (Utilities|Array|Add (LocalVariables|GetLargerThanPivot) _array_element)
        (else
          (Utilities|Array|Add (LocalVariables|GetSmallerThanPivot) _array_element))))
    ;[0.15 0.15 0.15 0.5] Recursively call Quicksort on both new arrays and append the results on either side of the 'pivot'
    (bind _output_list (CallFunction|Quicksort (LocalVariables|GetSmallerThanPivot)))
    (bind _output_get_2 (LocalVariables|SetOut _output_list))
    (Utilities|Array|AppendArray _output_get_2 (Utilities|Array|MakeArray (LocalVariables|GetPivot)))
    (bind _output_list_2 (CallFunction|Quicksort (LocalVariables|GetLargerThanPivot)))
    (Utilities|Array|AppendArray _output_get_2 _output_list_2)
    (return (LocalVariables|GetOut))
    (else
      (return (LocalVariables|GetArray)))))

(fn GatherCombattants
  (bind _outactors (Actor|GetAllActorsOfClass "/Game/Blueprints/BP_Basecharacter.BP_Basecharacter_C"))
  (Variables|Default|SetCombatants _outactors)
  (for _array_element (Variables|Default|GetCombatants)
    (Variables|/Game/Blueprints/BP_Basecharacter.BP_Basecharacter_C|SetInitiative _array_element (+ (Math|Random|RandomInteger 19) 1)))
  (bind _output_list (CallFunction|Quicksort (Variables|Default|GetCombatants)))
  (bind _output_get (Variables|Default|SetCombatants _output_list))
  (return _output_get))

(fn CombattantDied
  ;[0.15 0.15 0.15 0.5] Get remaining combatants
  (bind _outactors (Actor|GetAllActorsOfClass "/Game/Blueprints/BP_Basecharacter.BP_Basecharacter_C"))
  (bind _output_get (LocalVariables|SetRemainingCombatants _outactors))
  (Variables|Default|SetFactionHasWon true)
  ;[0.15 0.15 0.15 0.5] Get the current combatant so we can continue from them later if need be
  (LocalVariables|SetCurrentCombatant (Utilities|Array|Get(acopy) (Variables|Default|GetCombatants) (Variables|Default|GetTurnIndex)))
  ;[0.15 0.15 0.15 0.5] Check if all remaining combatants share a class
  (bind (_array_element _array_index) (Utilities|Array|ForEachLoopwithBreak _output_get)
    (:LoopBody
      (if (Utilities|Array|IsValidIndex (LocalVariables|GetRemainingCombatants) (+ _array_index 1))
        (Variables|Default|SetFactionHasWon (and (== (Utilities|GetClass _array_element) (Utilities|GetClass (Utilities|Array|Get(acopy) (LocalVariables|GetRemainingCombatants) (+ _array_index 1)))) (Variables|Default|GetFactionHasWon)))))
    (:Completed
      (if (Variables|Default|GetFactionHasWon)
        ;[0.15 0.15 0.15 0.5] Check which faction is alive and print corresponding message
        (Utilities|Casting|CastToBP_PlayerCharacter (Utilities|Array|Get(acopy) (LocalVariables|GetRemainingCombatants))
          (:then
            (Development|PrintString "Player Wins!"))
          (:CastFailed
            (Development|PrintString "Enemies win")))
        (return)
        (else
          ;[0.15 0.15 0.15 0.5] Prune null references and go to next turn
          (bind _output_get_2 (CallFunction|GatherCombattants))
          (Variables|Default|SetTurnIndex (Utilities|Array|FindItem _output_get_2 (LocalVariables|GetCurrentCombatant)))
          (CallFunction|AdvanceTurn)
          (return))))))