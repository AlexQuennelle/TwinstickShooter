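; Base character Blueprint for turn-based combat, holding Health and a reference to the BP_TurnBased game mode cached on BeginPlay.
; ApplyHealthChange adds a delta to Health through a math expression and returns IsDead, which tests whether Health is at or below zero.
; Die notifies the game mode through CombattantDied but is not called by the health logic here.
; StartTurn is an empty stub.
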(event EventBeginPlay
  (bind _asbp_turn_based (Utilities|Casting|CastToBP_TurnBased (Game|GetGameMode)))
  (Variables|Default|SetGamemode _asbp_turn_based))

(fn ConstructionScript)

(fn IsDead
  (return (|({A6E23125-4DB0-64BA-72F5-B193510976C9}<=0))))

(fn ApplyHealthChange
  (params (Delta :type Float%20%28double-precision%29))
  (Variables|BaseCharacter|SetHealth (|({A6E23125-4DB0-64BA-72F5-B193510976C9}+Delta) Delta))
  (return (CallFunction|IsDead)))

(fn StartTurn
  (return))

(fn Die
  (Default|CombattantDied (Variables|Default|GetGamemode))
  (return))